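; BP_FireBall is a fireball projectile that flies out and returns like a boomerang to a target actor.
; On authority only, one timeline lerps it forward along its facing to an apex at the travel distance.
; A second timeline then lerps it from the apex to ReturnToActor's live location.
; Once within explode distance of that actor during the return, it calls OnHit and destroys itself.
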(event `self.StartOutgoingTimeLine`
  (`/Engine/EditorBlueprintResources/ActorMacros.Switch Has Authority`
    (:`Authority`
      (set `self.InitLocation` (`self.K2_GetActorLocation`))
      (set `self.ApexLocation` (+ (`self.InitLocation`) (* (`self.GetActorForwardVector`) (`self.TravelDistance`))))
      (bind (_direction _outgoingtrack) (`Timeline|OutgoingTimeLine` :!via `PlayFromStart`)
        (:`Update`
          (`self.K2_SetActorLocation` (`KismetMathLibrary.VLerp` (`self.InitLocation`) (`self.ApexLocation`) _outgoingtrack)))
        (:`Finished`
          (bind (_direction_2 _retutningtrack) (`Timeline|ReturningTimeLine` :!via `PlayFromStart`)
            (:`Update`
              (bind _returntoactor (`self.ReturnToActor`)
                (:`then`
                  (`self.K2_SetActorLocation` (`KismetMathLibrary.VLerp` (`self.ApexLocation`) (`self.K2_GetActorLocation` _returntoactor) _retutningtrack))
                  (bind _returntoactor_2 (`self.ReturnToActor`)
                    (:`then`
                      (if (<= (`KismetMathLibrary.Vector_Distance` (`self.K2_GetActorLocation` _returntoactor_2) (`self.K2_GetActorLocation`)) (`self.ExplodeDistance`))
                        (`self.OnHit`)
                        (`self.K2_DestroyActor`)))
                    (:`else`)))
                (:`else`)))))))))

(fn `UserConstructionScript`)