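; BP_FadeActor is an actor that fades its static mesh out and back in through a material parameter.
; Construction caches the original materials and creates dynamic instances from a list of fade materials.
; FadeOut swaps in those instances and plays a timeline driving their "Fade" scalar, while Fadein reverses it.
; When the timeline finishes with Fade at 1 or above, the original materials are restored.
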(event `/Game/BP/Interface/BI_Fade.FadeOut`
  (`self.SetMaterialsByDynamicInstances`)
  (bind (_direction _fade) (`Timeline|FadeTimeLine` :!label _label)
    (:`Update`
      (for _array_element (`self.DynamicMaterials`)
        (`MaterialInstanceDynamic.SetScalarParameterValue` _array_element "Fade" _fade)))
    (:`Finished`
      (if (>= _fade 1.0)
        (`self.ResetMaterails`)))))

(event `/Game/BP/Interface/BI_Fade.FadeIn`
  (goto _label :!via `Reverse`))

(fn `ResetMaterails`
  (for (_array_element _array_index) (`self.OriginMaterials`)
    (`PrimitiveComponent.SetMaterial` (`self.StaticMesh`) _array_index _array_element)))

(fn `SetMaterialsByDynamicInstances`
  (for (_array_element _array_index) (`self.DynamicMaterials`)
    (`PrimitiveComponent.SetMaterial` (`self.StaticMesh`) _array_index _array_element)))

(fn `UserConstructionScript`
  (`KismetArrayLibrary.Array_Clear` (`self.DynamicMaterials`))
  (set `self.OriginMaterials` (`MeshComponent.GetMaterials` (`self.StaticMesh`)))
  (for _array_element (`self.FadeMaterialsInstance`)
    (bind _returnvalue (`KismetMaterialLibrary.CreateDynamicMaterialInstance` _array_element))
    (`KismetArrayLibrary.Array_AddUnique` (`self.DynamicMaterials`) _returnvalue)))