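; Enemy gameplay ability that summons random minions with default controllers, played with the shaman summon montage.
; On activation it shuffles the spawn locations, shows a ground Niagara effect at each and caches the avatar's rotation.
; The montage's attack event starts a Delay-driven loop that staggers the spawns, drawing a debug sphere and incrementing the summoner's minion count for each.
; The graph never calls EndAbility.
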(event `self.K2_ActivateAbility`
  (bind _output (`|GetArrayItem` (`self.SpawnLocations`) (`self.SpawnLocationIndex`)))
  (bind _output_get (set `self.SpawnLocations` (`self.GetSpawnLocations`)))
  (`KismetArrayLibrary.Array_Shuffle` _output_get)
  (`|ExecutionSequence`
    (:`then_0`
      (for _array_element (`self.SpawnLocations`)
        (`NiagaraFunctionLibrary.SpawnSystemAtLocation` "/Game/Assets/Effects/Combat/NS_GroundSummon.NS_GroundSummon" _array_element (struct) (1.0 1.0 1.0) true true "AutoRelease"))
      (`AbilityTask_PlayMontageAndWait.CreatePlayMontageAndWaitProxy` "None" "/Game/Assets/Enemies/Shaman/Animations/AM_Shaman_Summon.AM_Shaman_Summon"
        (:`then`
          (`AbilityTask_WaitGameplayEvent.WaitGameplayEvent` (struct :`TagName` "Montage.Attack.1") null true
            (:`EventReceived`
              (if (< (`self.SpawnLocationIndex`) (`KismetArrayLibrary.Array_Length` (`self.SpawnLocations`))) :!label _label
                (`KismetSystemLibrary.DrawDebugSphere` _output 25.0 12 (struct :`R` 1.0 :`G` 0.012392 :`B` 0.872994 :`A` 1.0) 3.0)
                (bind _returnvalue (`|SpawnActorFromClass` (`self.GetRandomMinionClass`) (`KismetMathLibrary.MakeTransform` (+ _output (0.0 0.0 50.0)) (`self.CurrentRotation`)) "AdjustIfPossibleButAlwaysSpawn" "MultiplyWithRoot" null null))
                (`Pawn.SpawnDefaultController` _returnvalue)
                (message `CombatInterface.IncrementMinionCount` (`self.GetAvatarActorFromActorInfo`) 1)
                (`/Engine/EditorBlueprintResources/StandardMacros.IncrementInt` (`self.SpawnLocationIndex`)
                  (:`  `
                    (`KismetSystemLibrary.Delay` 0.2)
                    (goto _label)))))))))
    (:`then_1`
      (set `self.CurrentRotation` (`Actor.K2_GetActorRotation` (`self.GetAvatarActorFromActorInfo`))))))