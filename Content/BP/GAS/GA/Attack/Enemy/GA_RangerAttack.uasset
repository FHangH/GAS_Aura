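; GA_RangerAttack is an enemy gameplay ability for a ranged attack that fires a projectile at the avatar's combat target.
; Through the combat interface it turns the avatar to face the target and plays a random tagged attack montage.
; The montage's tag is awaited as a gameplay event, which spawns the projectile toward the target's current location and ends the ability.
; Montage completion, interruption or cancellation also ends it.
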(event `self.K2_ActivateAbility`
  (bind _returnvalue (`self.GetAvatarActorFromActorInfo`))
  (bind _returnvalue_2 (`self.GetAvatarActorFromActorInfo`))
  (bind _ascombat_interface (cast `CombatInterface` _returnvalue_2)
    (:`then`
      (bind _returnvalue_3 (message `EnemyInterface.GetCombatTarget` _returnvalue_2))
      (`CombatInterface.UpdateFacingTarget` _ascombat_interface (`Actor.K2_GetActorLocation` _returnvalue_3))
      (bind _returnvalue_4 (message `CombatInterface.GetAttackMontages` (`self.GetAvatarActorFromActorInfo`)))
      (bind _output_get (set `self.TaggedMontage` (`self.GetRandomTaggedMontage` _returnvalue_4)))
      (bind (_montage _montagetag) (break `TaggedMontage` _output_get))
      (`AbilityTask_PlayMontageAndWait.CreatePlayMontageAndWaitProxy` "None" _montage 1.0 "None" false
        (:`then`
          (`AbilityTask_WaitGameplayEvent.WaitGameplayEvent` _montagetag null true
            (:`EventReceived`
              (message `CombatInterface.GetCombatSocketLocation` _returnvalue _montagetag)
              (bind _returnvalue_5 (message `EnemyInterface.GetCombatTarget` _returnvalue))
              (`self.SpawnProjectile` (`Actor.K2_GetActorLocation` _returnvalue_5))
              (`self.K2_EndAbility`))))
        (:`OnCompleted`
          (`self.K2_EndAbility` :!label _label))
        (:`OnInterrupted`
          (goto _label))
        (:`OnCancelled`
          (goto _label))))
    (:`CastFailed`
      (`self.K2_EndAbility`))))