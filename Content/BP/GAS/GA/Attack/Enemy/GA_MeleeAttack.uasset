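; Gameplay Ability for an enemy melee attack that turns the avatar toward its combat target and plays a random tagged attack montage.
; The montage's tag gameplay event triggers a small radius check for live players at the matching combat socket, obtained through CombatInterface.
; Non-friends take damage and spawn blood effects, with one impact sound on any hit.
; The ability ends after that check, on a friendly overlap, or when the montage finishes.
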(event `self.K2_ActivateAbility`
  (bind _returnvalue (`self.GetAvatarActorFromActorInfo`))
  (bind _returnvalue_2 (`self.GetAvatarActorFromActorInfo`))
  (set `self.HasHitTarget` false)
  (bind _ascombat_interface (cast `CombatInterface` _returnvalue_2)
    (:`then`
      (bind _returnvalue_3 (message `EnemyInterface.GetCombatTarget` _returnvalue_2))
      (`CombatInterface.UpdateFacingTarget` _ascombat_interface (`Actor.K2_GetActorLocation` _returnvalue_3))
      (bind _returnvalue_4 (message `CombatInterface.GetAttackMontages` (`self.GetAvatarActorFromActorInfo`)))
      (bind _output_get (set `self.TaggedMontage` (`self.GetRandomTaggedMontage` _returnvalue_4)))
      (bind (_montage _montagetag _impactsound) (break `TaggedMontage` _output_get))
      (`AbilityTask_PlayMontageAndWait.CreatePlayMontageAndWaitProxy` "None" _montage 1.0 "None" false
        (:`then`
          (`AbilityTask_WaitGameplayEvent.WaitGameplayEvent` _montagetag null true
            (:`EventReceived`
              (bind _returnvalue_5 (message `CombatInterface.GetCombatSocketLocation` _returnvalue _montagetag))
              (for _array_element (`AuraAbilitySystemFuncLibrary.GetLivePlayersWithRadius` _returnvalue (`|MakeArray` _returnvalue) 50.0 _returnvalue_5)
                (if (`AuraAbilitySystemFuncLibrary.IsNotFriend` (`self.GetAvatarActorFromActorInfo`) _array_element)
                  (`self.CauseDamage` _array_element)
                  (set `self.HasHitTarget` true)
                  (bind _returnvalue_6 (message `CombatInterface.GetBloodEffect` _array_element))
                  (`NiagaraFunctionLibrary.SpawnSystemAtLocation` _returnvalue_6 _returnvalue_5 (struct) (1.0 1.0 1.0) true true "AutoRelease")
                  (else
                    (`self.K2_EndAbility` :!label _label))))
              (if (`self.HasHitTarget`)
                (`GameplayStatics.PlaySoundAtLocation` _impactsound _returnvalue_5 (struct) 1.0 1.0 0.0 null null null null)
                (goto _label)
                (else
                  (goto _label))))))
        (:`OnCompleted`
          (`self.K2_EndAbility` :!label _label_2))
        (:`OnInterrupted`
          (goto _label_2))
        (:`OnCancelled`
          (goto _label_2))))
    (:`CastFailed`
      (`self.K2_EndAbility`))))

(event `self.K2_OnEndAbility`
  (params (bWasCancelled :type Boolean))
  (set `self.HasHitTarget` false))