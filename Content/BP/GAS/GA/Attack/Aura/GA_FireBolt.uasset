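; GA_FireBolt is a gameplay ability that casts a fire bolt projectile toward the point under the mouse.
; After committing, it gets target data under the mouse, turns the avatar to face that location through CombatInterface and plays the cast montage.
; A montage gameplay event times the projectile spawn from the weapon socket, and the ability ends when the montage completes, blends out, is interrupted or is cancelled.
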(event `self.K2_ActivateAbility`
  (bind _returnvalue (`self.K2_CommitAbility`))
  (if _returnvalue
    (bind (_asynctaskproxy _datahandle) (`AT_TargetDataUnderMouse.CreateTargetDataUnderMouse`)
      (:`ValidData`
        (set `self.Location` (`.Location` (`GameplayStatics.BreakHitResult` (`AbilitySystemBlueprintLibrary.GetHitResultFromTargetData` _datahandle))))
        (bind _ascombat_interface (cast `CombatInterface` (`self.GetAvatarActorFromActorInfo`))
          (:`then`
            (`CombatInterface.UpdateFacingTarget` _ascombat_interface (`self.Location`))
            (`AbilityTask_PlayMontageAndWait.CreatePlayMontageAndWaitProxy` "None" "/Game/Assets/Characters/Aura/Animations/Abilities/AM_Cast_FireBolt.AM_Cast_FireBolt" 1.0 "None" false
              (:`then`
                (`AbilityTask_WaitGameplayEvent.WaitGameplayEvent` (struct :`TagName` "Event.Montage.FireBolt") null true
                  (:`EventReceived`
                    (`self.SpawnProjectile` (`self.Location`) (`BlueprintGameplayTagLibrary.MakeLiteralGameplayTag` (struct :`TagName` "CombatSocket.Weapon"))))))
              (:`OnCompleted`
                (`self.K2_EndAbility` :!label _label))
              (:`OnBlendOut`
                (goto _label))
              (:`OnInterrupted`
                (goto _label))
              (:`OnCancelled`
                (goto _label))))
          (:`CastFailed`
            (`self.K2_EndAbility`)))))))

(event `self.K2_OnEndAbility`
  (params (bWasCancelled :type Boolean)))