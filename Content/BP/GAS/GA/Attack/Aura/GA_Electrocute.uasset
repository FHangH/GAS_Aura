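; GA_Electrocute is a channeled lightning Gameplay Ability that fires a beam at the target under the mouse and chains to additional targets.
; A montage event locks movement, adds looping shock cues and unpauses a damage timer.
; Each tick commits cost and applies SetByCaller lightning damage, ending when cost fails or the target is dead.
; Input release or montage cancellation restores movement and cursor, removes cues and ends the ability.
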(event `self.K2_ActivateAbility`
  (bind _returnvalue (`self.K2_CommitAbility`))
  (if (and _returnvalue (`KismetSystemLibrary.DoesImplementInterface` (`self.GetAvatarActorFromActorInfo`) "/Script/GAS_Aura.CombatInterface"))
    (bind (_asynctaskproxy _datahandle) (`AT_TargetDataUnderMouse.CreateTargetDataUnderMouse`)
      (:`then`
        (bind _returnvalue_2 (`KismetSystemLibrary.K2_SetTimerDelegate` (`|CreateDelegate` :!event `OnDamageAndCost`) (`self.DamageDeltaTime`) true))
        (bind _output_get (set `self.Timer_Damage` _returnvalue_2))
        (`KismetSystemLibrary.K2_PauseTimerHandle` _output_get))
      (:`ValidData`
        (`self.StoreMouseDataInfo` (`AbilitySystemBlueprintLibrary.GetHitResultFromTargetData` _datahandle))
        (`self.StoreOwners`)
        (message `CombatInterface.UpdateFacingTarget` (`self.GetAvatarActorFromActorInfo`) (`self.MouseHitLocation`))
        (set `PlayerController.bShowMouseCursor` false (`self.OwnerPlayerController`))
        (`self.K2_ExecuteGameplayCue` (struct :`TagName` "GameplayCue.ShockBurst"))
        (`AbilityTask_PlayMontageAndWait.CreatePlayMontageAndWaitProxy` "None" (`self.Montage_Electrocute`)
          (:`then`
            (`AbilityTask_WaitGameplayEvent.WaitGameplayEvent` (struct :`TagName` "Event.Montage.Electrocute") null true
              (:`then`
                (`AbilityTask_WaitInputRelease.WaitInputRelease` false
                  (:`OnRelease`
                    (`self.PrepareToEndAbility` :!label _label)
                    (if (`self.IsCharacter`)
                      (`GameplayCueFunctionLibrary.RemoveGameplayCueOnActor` (`self.MouseHitActor`) (struct :`TagName` "GameplayCue.ShockLoop") (`self.FirstTargetCueParams`))
                      (for _array_element (`self.AdditionalTargets`)
                        (`self.RemoveShockLoopCueFromAdditionalTarget` _array_element))
                      (else
                        (`GameplayCueFunctionLibrary.RemoveGameplayCueOnActor` (`self.GetAvatarActorFromActorInfo`) (struct :`TagName` "GameplayCue.ShockLoop") (`self.FirstTargetCueParams`))))
                    (`self.K2_EndAbility`))))
              (:`EventReceived`
                (`self.InShockLoop`)
                (`self.SpawnElectricBeam`)
                (`KismetSystemLibrary.K2_UnPauseTimerHandle` (`self.Timer_Damage`)))))
          (:`OnCancelled`
            (goto _label)))))
    (else
      (`self.K2_EndAbility`))))

(event `OnDamageAndCost`
  (bind _returnvalue (`self.K2_CommitAbilityCost` false))
  (if _returnvalue
    (if (`self.IsTargetDead`)
      (`self.ClearTimerAndEndAbility`)
      (else
        (`self.ApplyDamage`)))
    (else
      (`self.ClearTimerAndEndAbility`))))

(fn `AddShockLoopCueToAdditionalTarget`
  (params (AdditionalTarget :type "Actor Object Reference"))
  (locals (Target :type "Actor Object Reference"))
  (bind _target (`local.Target`))
  (bind _returnvalue (`AbilitySystemBlueprintLibrary.MakeGameplayCueParameters` 0.0 0.0 (struct) (struct) (struct) (struct) (struct) (`Actor.K2_GetActorLocation` _target) (0.0 0.0 0.0) null null _target null 1 1 (`Actor.RootComponent` (`self.MouseHitActor`))))
  (set `local.Target` AdditionalTarget)
  (`BlueprintMapLibrary.Map_Add` (`self.Map_AddiitonalActorToCueParams`) _target _returnvalue)
  (`GameplayCueFunctionLibrary.AddGameplayCueOnActor` (`local.Target`) (struct :`TagName` "GameplayCue.ShockLoop") _returnvalue))

(fn `ApplyDamage`
  (`self.ApplyDamageSingleTarget` (`self.MouseHitActor`))
  (for _array_element (`self.AdditionalTargets`)
    (`self.ApplyDamageSingleTarget` _array_element)))

(fn `ApplyDamageSingleTarget`
  (params (Target :type "Actor Object Reference"))
  (bind _returnvalue (`self.GetAbilitySystemComponentFromActorInfo`))
  (`/Engine/EditorBlueprintResources/StandardMacros.IsValid` Target
    (:`Is Valid`
      (bind _returnvalue_2 (`AbilitySystemBlueprintLibrary.AssignTagSetByCallerMagnitude` (`AbilitySystemComponent.MakeOutgoingSpec` _returnvalue (`self.DamageEffectClass`) (`KismetMathLibrary.Conv_IntToDouble` (`self.GetAbilityLevel`)) (`AbilitySystemComponent.MakeEffectContext` _returnvalue)) (struct :`TagName` "Damage.Lightning") (`self.GetDamageAtLevel`)))
      (`AbilitySystemComponent.BP_ApplyGameplayEffectSpecToSelf` (`AbilitySystemBlueprintLibrary.GetAbilitySystemComponent` Target) _returnvalue_2))))

(fn `ClearTimerAndEndAbility`
  (`KismetSystemLibrary.K2_ClearAndInvalidateTimerHandle` (`self.Timer_Damage`))
  (`self.PrepareToEndAbility`)
  (`self.K2_EndAbility`))

(fn `InShockLoop`
  (message `CombatInterface.SetInShockLoop` (`self.GetAvatarActorFromActorInfo`) true)
  (`CharacterMovementComponent.DisableMovement` (`Character.CharacterMovement` (`self.OwnerCharacter`))))

(fn `PrepareToEndAbility`
  (message `CombatInterface.SetInShockLoop` (`self.GetAvatarActorFromActorInfo`) false)
  (set `PlayerController.bShowMouseCursor` true (`self.OwnerPlayerController`))
  (`CharacterMovementComponent.SetMovementMode` (`Character.CharacterMovement` (`self.OwnerCharacter`)) "MOVE_Walking" 0))

(fn `RemoveShockLoopCueFromAdditionalTarget`
  (params (Key :type "Actor Object Reference (by ref)"))
  (bind (_value _returnvalue) (`BlueprintMapLibrary.Map_Find` (`self.Map_AddiitonalActorToCueParams`) Key))
  (if _returnvalue
    (`GameplayCueFunctionLibrary.RemoveGameplayCueOnActor` Key (struct :`TagName` "GameplayCue.ShockLoop") _value)))

(fn `SpawnElectricBeam`
  (locals (CueTarget :type "Actor Object Reference"))
  (`self.TraceFirstTarget` (`self.MouseHitLocation`))
  (bind _returnvalue (message `CombatInterface.GetWeaponMesh` (`self.OwnerCharacter`)))
  (set `self.FirstTargetCueParams` (`AbilitySystemBlueprintLibrary.MakeGameplayCueParameters` 0.0 0.0 (struct) (struct) (struct) (struct) (struct) (`self.MouseHitLocation`) (0.0 0.0 0.0) null null (`self.MouseHitActor`) null 1 1 _returnvalue))
  (set `self.IsCharacter` (`KismetSystemLibrary.DoesImplementInterface` (`self.MouseHitActor`) "/Script/GAS_Aura.CombatInterface"))
  (if (`self.IsCharacter`)
    (set `local.CueTarget` (`self.MouseHitActor`))
    (else
      (set `local.CueTarget` (`self.GetAvatarActorFromActorInfo`))))
  (`GameplayCueFunctionLibrary.AddGameplayCueOnActor` (`local.CueTarget`) (struct :`TagName` "GameplayCue.ShockLoop") (`self.FirstTargetCueParams`))
  (if (`self.IsCharacter`)
    (bind _output_get (set `self.AdditionalTargets` (`self.StoreAdditionalTargets`)))
    (for _array_element _output_get
      (`self.AddShockLoopCueToAdditionalTarget` _array_element)))
  (return))