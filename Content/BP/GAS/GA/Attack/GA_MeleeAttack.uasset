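; Gameplay ability for a melee attack by an avatar that implements CombatInterface.
; It turns the avatar toward its combat target and plays a random attack montage, then waits for that montage's gameplay event tag.
; On the event, it damages live players within a small sphere at the tagged combat socket, draws debug spheres on them, and ends.
; The ability also ends when the montage finishes or is interrupted.
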(event `self.K2_ActivateAbility`
  (bind _returnvalue (`self.GetAvatarActorFromActorInfo`))
  (bind _returnvalue_2 (`self.GetAvatarActorFromActorInfo`))
  (bind _ascombat_interface (cast `CombatInterface` _returnvalue_2)
    (:`then`
      (bind _returnvalue_3 (message `EnemyInterface.GetCombatTarget` _returnvalue_2))
      (`CombatInterface.UpdateFacingTarget` _ascombat_interface (`Actor.K2_GetActorLocation` _returnvalue_3))
      (bind _returnvalue_4 (message `CombatInterface.GetAttackMontages` (`self.GetAvatarActorFromActorInfo`)))
      (bind (_montage _montagetag) (break `TaggedMontage` (`KismetArrayLibrary.Array_Random` _returnvalue_4)))
      (`AbilityTask_PlayMontageAndWait.CreatePlayMontageAndWaitProxy` "None" _montage
        (:`then`
          (`AbilityTask_WaitGameplayEvent.WaitGameplayEvent` _montagetag null true
            (:`EventReceived`
              (bind _returnvalue_5 (message `CombatInterface.GetCombatSocketLocation` _returnvalue _montagetag))
              (for _array_element (`AuraAbilitySystemFuncLibrary.GetLivePlayersWithRadius` _returnvalue (`|MakeArray` _returnvalue) 30.0 _returnvalue_5)
                (`KismetSystemLibrary.DrawDebugSphere` (`Actor.K2_GetActorLocation` _array_element) 30.0 12 (struct :`R` 0.018688 :`G` 1.0 :`A` 1.0) 1.0)
                (`self.CauseDamage` _array_element))
              (`self.K2_EndAbility`))))
        (:`OnCompleted`
          (`self.K2_EndAbility` :!label _label))
        (:`OnBlendOut`
          (goto _label))
        (:`OnInterrupted`
          (goto _label))
        (:`OnCancelled`
          (goto _label))))
    (:`CastFailed`
      (`self.K2_EndAbility`))))