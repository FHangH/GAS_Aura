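; GA_ManaSiphon is a Gameplay Ability filed under passive spells that currently only prints debug messages when it activates and ends.
; ActivateAbility and OnEndAbility both call a PrintLog helper, which shows the object's name with an activated or end label as colored, timed text.
; The file contains no mana siphon logic, effect application or explicit end-ability call.
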(event `self.K2_ActivateAbility`
  (`self.PrintLog` true (struct :`G` 0.051529 :`B` 1.0 :`A` 1.0) 5.0 self))

(event `self.K2_OnEndAbility`
  (params (bWasCancelled :type Boolean))
  (`self.PrintLog` false (struct :`G` 0.051529 :`B` 1.0 :`A` 1.0) 5.0 self))

(fn `PrintLog`
  (params (IsActive :type Boolean) (TextColor :type "LinearColor Structure") (Duration :type "Float (single-precision)") (Object :type "Object Object Reference"))
  (bind _returnvalue (`KismetSystemLibrary.GetObjectName` Object))
  (if IsActive
    (`KismetSystemLibrary.PrintText` (`|FormatText` "{name} -- Activaed" _returnvalue) true true TextColor Duration)
    (else
      (`KismetSystemLibrary.PrintText` (`|FormatText` "{name} -- End" _returnvalue) true true TextColor Duration))))