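; Base enemy character Blueprint that supplies spawn, dissolve and facing behavior.
; On BeginPlay a timeline drives uniform mesh scale for a spawn effect.
; Separate body and weapon timelines animate the Dissolve scalar on dynamic materials passed into their events.
; UpdateFacingTarget feeds a location to Motion Warping as the FacingTarget warp target.
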(event `self.ReceiveBeginPlay`
  (bind (_direction _scaletrack) (`Timeline|SpawnTimeline` :!via `PlayFromStart`)
    (:`Update`
      (`SceneComponent.SetRelativeScale3D` (`self.Mesh`) (`KismetMathLibrary.MakeVector` _scaletrack _scaletrack _scaletrack)))))

(event `self.StartBodyDissolveTimeLine`
  (params (DynamicMatIns :type "MaterialInstanceDynamic Object Reference"))
  (bind (_direction _newtrack_0) (`Timeline|DissolveTimeline` :!via `PlayFromStart`)
    (:`Update`
      (`MaterialInstanceDynamic.SetScalarParameterValue` DynamicMatIns "Dissolve" _newtrack_0))))

(event `self.StartWeaponDissolveTimeLine`
  (params (DynamicMatIns :type "MaterialInstanceDynamic Object Reference"))
  (bind (_direction _newtrack_0) (`Timeline|Timeline` :!via `PlayFromStart`)
    (:`Update`
      (`MaterialInstanceDynamic.SetScalarParameterValue` DynamicMatIns "Dissolve" _newtrack_0))))

(event `CombatInterface.UpdateFacingTarget`
  (params (TargetLocation :type "Vector Structure (by ref)"))
  (`MotionWarpingComponent.AddOrUpdateWarpTargetFromLocation` (`self.MotionWarping`) "FacingTarget" TargetLocation))

(fn `UserConstructionScript`)